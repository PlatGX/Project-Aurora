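; Base weapon actor that takes its stats from a data table, in an early prototype state.
; ChangeWeapon looks up a row in WeaponTable by ID, stores it in CurrentWeapon and prints the equipped weapon's name.
; BeginPlay calls it with a hardcoded default ID; no mesh, firing or other behavior is scripted, and leftover table-query nodes are unconnected.
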(event `self.ReceiveBeginPlay`
  (`self.ChangeWeapon` "1001"))

(fn `ChangeWeapon`
  (params (WeaponID :type Name))
  (bind _returnvalue (`|GetDataTableRow` (`self.WeaponTable`) WeaponID)
    (:`then`
      (bind _output_get (set `self.CurrentWeapon` _returnvalue))
      (`KismetSystemLibrary.PrintString` (`KismetStringLibrary.Concat_StrStr` "Equipped the " (`.Name_2_6376CDF14D27DFA0E7F2198854CD7058` (break `/Game/Developer/Jarvis/CharacterSystem/SWeaponStats` _output_get)))))))

(fn `UserConstructionScript`)